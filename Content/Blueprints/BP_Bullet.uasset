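; BP_Bullet is a projectile actor that produces impact effects when it hits something, then destroys itself.
; On hit, it attaches a randomly sized, temporary bullet-hole decal to the struck component, plays an impact sound and spawns Niagara smoke and shards aligned to the surface normal.
; It stores the shard system's location for PlayParticleCollisionSound, which plays a brick impact sound there but is not called within this Blueprint.
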(event `self.ReceiveHit`
  (params (MyComp :type "PrimitiveComponent Object Reference") (Other :type "Actor Object Reference") (OtherComp :type "PrimitiveComponent Object Reference") (bSelfMoved :type Boolean) (HitLocation :type "Vector Structure") (HitNormal :type "Vector Structure") (NormalImpulse :type "Vector Structure") (Hit :type "HitResult Structure (by ref)"))
  (bind _returnvalue (`KismetMathLibrary.Conv_VectorToRotator` HitNormal))
  (bind _bullet (`self.Bullet`))
  (`GameplayStatics.SpawnDecalAttached` "/Game/UI+2D/Images/MAT_Bullet_Hole.MAT_Bullet_Hole" (`KismetMathLibrary.MakeVector` (`KismetMathLibrary.RandomFloatInRange` 7.5 11.5) 5.0 5.0) OtherComp "None" HitLocation _returnvalue "KeepWorldPosition" 30.0)
  (`GameplayStatics.PlaySoundAtLocation` "/Game/Audio/SC_Bullet_Impacts.SC_Bullet_Impacts" HitLocation (struct) 1.0 1.0 0.0 null null null null)
  (`NiagaraFunctionLibrary.SpawnSystemAtLocation` "/Game/VFX/NS_Impact_Smoke.NS_Impact_Smoke" HitLocation _returnvalue)
  (bind _returnvalue_2 (`NiagaraFunctionLibrary.SpawnSystemAtLocation` "/Game/VFX/NS_Impact_Shards.NS_Impact_Shards" HitLocation _returnvalue))
  (set `self.Particle Collision Location` (`SceneComponent.K2_GetComponentLocation` _returnvalue_2))
  (`SceneComponent.SetVisibility` _bullet false false)
  (`PrimitiveComponent.SetCollisionEnabled` _bullet "NoCollision")
  (`self.K2_DestroyActor`))

(fn `Play Particle Collision Sound`
  (`GameplayStatics.PlaySoundAtLocation` "/Game/Audio/SC_Brick_Impact.SC_Brick_Impact" (`self.Particle Collision Location`) (struct) 1.0 1.0 0.0 null null null null))

(fn `UserConstructionScript`)