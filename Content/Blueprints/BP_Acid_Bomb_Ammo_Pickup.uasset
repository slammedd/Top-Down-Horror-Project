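; Acid bomb ammo pickup that grants one round to the third-person character on overlap, only if the acid bomb is unlocked.
; The box overlap increments the character's clamped ammo count and plays a pickup sound.
; If the HUD's acid bomb element has not faded, it fades in, the pickup's meshes and light hide, and a short delay precedes the fade-out.
; The actor then destroys itself.
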(event `self.Box.OnComponentBeginOverlap`
  (params (OverlappedComponent :type "PrimitiveComponent Object Reference") (OtherActor :type "Actor Object Reference") (OtherComp :type "PrimitiveComponent Object Reference") (OtherBodyIndex :type Integer) (bFromSweep :type Boolean) (SweepResult :type "HitResult Structure (by ref)"))
  (bind _asbp_third_person_character (cast `/Game/Blueprints/BP_ThirdPersonCharacter` OtherActor))
  (if (`/Game/Blueprints/BP_ThirdPersonCharacter.Acid Bomb Unlocked` _asbp_third_person_character)
    (set `/Game/Blueprints/BP_ThirdPersonCharacter.Acid Bomb Ammo` (`KismetMathLibrary.Clamp` (+ (`/Game/Blueprints/BP_ThirdPersonCharacter.Acid Bomb Ammo` _asbp_third_person_character) 1) 0 99) _asbp_third_person_character)
    (`GameplayStatics.PlaySoundAtLocation` "/Game/Audio/SC_Acid_Bomb_Pickup.SC_Acid_Bomb_Pickup" (`SceneComponent.K2_GetComponentLocation` (`self.Container`)) (struct) 1.0 1.0 0.0 null null null null)
    (bind _hud (`/Game/Blueprints/BP_ThirdPersonCharacter.HUD` _asbp_third_person_character))
    (if (not (`/Game/UI+2D/WB_HUD.Has Faded AB` _hud))
      (`/Game/UI+2D/WB_HUD.Fade In AB` _hud)
      (`SceneComponent.SetVisibility` (`self.testube_done_not_opaque_pCylinder10`) false false)
      (`SceneComponent.SetVisibility` (`self.testube_done_not_opaque_pCylinder8`) false false)
      (`SceneComponent.SetVisibility` (`self.testube_done_not_opaque_pCylinder9`) false false)
      (`SceneComponent.SetVisibility` (`self.PointLight`) false false)
      (`KismetSystemLibrary.Delay` 2.0)
      (`/Game/UI+2D/WB_HUD.Fade Out AB` _hud))
    (`self.K2_DestroyActor`)))

(fn `UserConstructionScript`)