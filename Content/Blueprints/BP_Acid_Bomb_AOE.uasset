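; Acid bomb area-of-effect actor that toggles the footstep sound override on BP_ThirdPersonCharacter as it enters or leaves the AOE component.
; BeginPlay traces 200 units upward, but sets actor Z from a hit result built only from the trace's boolean, not its actual impact point.
; A delayed event removes the AOE component after a few seconds.
; A longer Lifetime event destroys the actor, though nothing here calls it.
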(event `Lifetime`
  (`KismetSystemLibrary.Delay` 8.0)
  (`self.K2_DestroyActor`))

(event `Collision Timer`
  (`KismetSystemLibrary.Delay` 6.5)
  (`ActorComponent.K2_DestroyComponent` (`self.AOE`)))

(event `self.ReceiveBeginPlay`
  (bind (_returnvalue_x _returnvalue_y) (`KismetMathLibrary.BreakVector` (`self.K2_GetActorLocation`)))
  (bind _returnvalue (`self.K2_GetActorLocation`))
  (`self.Collision Timer`)
  (bind (_outhit _returnvalue_2) (`KismetSystemLibrary.LineTraceSingle` :`Start` _returnvalue :`End` (- _returnvalue (0.0 0.0 -200.0)) :`TraceChannel` "TraceTypeQuery1" :`DrawDebugType` "ForOneFrame"))
  (`self.K2_SetActorLocation` (`KismetMathLibrary.MakeVector` _returnvalue_x _returnvalue_y (.z (`.ImpactPoint` (`GameplayStatics.BreakHitResult` (`GameplayStatics.MakeHitResult` _returnvalue_2)))))))

(event `self.AOE.OnComponentBeginOverlap`
  (params (OverlappedComponent :type "PrimitiveComponent Object Reference") (OtherActor :type "Actor Object Reference") (OtherComp :type "PrimitiveComponent Object Reference") (OtherBodyIndex :type Integer) (bFromSweep :type Boolean) (SweepResult :type "HitResult Structure (by ref)"))
  (bind _asbp_third_person_character (cast `/Game/Blueprints/BP_ThirdPersonCharacter` OtherActor))
  (set `/Game/Blueprints/BP_ThirdPersonCharacter.Override Footstep Sounds` true _asbp_third_person_character))

(event `self.AOE.OnComponentEndOverlap`
  (params (OverlappedComponent :type "PrimitiveComponent Object Reference") (OtherActor :type "Actor Object Reference") (OtherComp :type "PrimitiveComponent Object Reference") (OtherBodyIndex :type Integer))
  (bind _asbp_third_person_character (cast `/Game/Blueprints/BP_ThirdPersonCharacter` OtherActor))
  (set `/Game/Blueprints/BP_ThirdPersonCharacter.Override Footstep Sounds` false _asbp_third_person_character))

(fn `UserConstructionScript`)